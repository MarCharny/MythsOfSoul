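; Dialogue NPC actor that prompts a nearby player to talk and shows an Anubis dialogue widget.
; Its trigger radius shows the press-E prompt, registers as BP_Player's CurrentNPC and enables per-tick turning toward the player; leaving clears this.
; StartDialogue swaps the prompt for the widget in Game-and-UI input and binds its response event.
; Responses only print debug text and restore game input; the talking montage function is an empty stub.
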(event `self.ReceiveBeginPlay`)

(event `self.ReceiveTick`
  (params (DeltaSeconds :type "Float (single-precision)"))
  (if (`self.isPlayerInRange`)
    (`self.RotateToPlayer`)))

(event `self.DialogTriggerRadius.OnComponentBeginOverlap`
  (params (OverlappedComponent :type "PrimitiveComponent Object Reference") (OtherActor :type "Actor Object Reference") (OtherComp :type "PrimitiveComponent Object Reference") (OtherBodyIndex :type Integer) (bFromSweep :type Boolean) (SweepResult :type "HitResult Structure (by ref)"))
  (bind _asbp_third_person_character (cast `/Game/ThirdPerson/Blueprints/BP_Player` OtherActor))
  (set `self.TargetPlayer` _asbp_third_person_character)
  (set `self.isPlayerInRange` true)
  (`self.PlayTalkingAnimMontage`)
  (bind _returnvalue (`|CreateWidget` "/Game/UI/Dialogs/WBP_PressEToDialogue.WBP_PressEToDialogue_C"))
  (`UserWidget.AddToViewport` _returnvalue 0)
  (set `self.PressEToDialogueRef` _returnvalue)
  (bind _asbp_third_person_character_2 (cast `/Game/ThirdPerson/Blueprints/BP_Player` (`GameplayStatics.GetPlayerCharacter` 0)))
  (set `/Game/ThirdPerson/Blueprints/BP_Player.CurrentNPC` self _asbp_third_person_character_2))

(event `self.DialogTriggerRadius.OnComponentEndOverlap`
  (params (OverlappedComponent :type "PrimitiveComponent Object Reference") (OtherActor :type "Actor Object Reference") (OtherComp :type "PrimitiveComponent Object Reference") (OtherBodyIndex :type Integer))
  (bind _dialogueuiref (`self.DialogueUIRef`))
  (bind _pressetodialogueref (`self.PressEToDialogueRef`))
  (cast `/Game/ThirdPerson/Blueprints/BP_Player` OtherActor)
  (set `self.TargetPlayer` null)
  (set `self.isPlayerInRange` false)
  (if (`KismetSystemLibrary.IsValid` _dialogueuiref)
    (`Widget.RemoveFromParent` _dialogueuiref)
    (set `self.PressEToDialogueRef` null :!label _label)
    (set `self.DialogueUIRef` null)
    (bind _asbp_third_person_character (cast `/Game/ThirdPerson/Blueprints/BP_Player` (`GameplayStatics.GetPlayerCharacter` 0)))
    (set `/Game/ThirdPerson/Blueprints/BP_Player.CurrentNPC` null _asbp_third_person_character)
    (set `/Game/ThirdPerson/Blueprints/BP_Player.InDialogue` false _asbp_third_person_character)
    (`self.RestorePlayerInput`)
    (elif (`KismetSystemLibrary.IsValid` _pressetodialogueref)
      (`Widget.RemoveFromParent` _pressetodialogueref)
      (goto _label))))

(event `Start Dialogue`
  (`self.Create Dialog Widget`)
  (add `/Game/UI/Dialogs/WBP_Dialogue_Anubis.OnResponseSelected` (`self.DialogueUIRef`) (delegate `HandleResponse`)))

(event `HandleResponse`
  (params (ResponseIndex :type Integer))
  (`KismetSystemLibrary.PrintText` "HIIIII")
  (switch `int` ResponseIndex
    (:`0`
      (`KismetSystemLibrary.PrintText` "Вы нажали кнопку 1"))
    (:`1`
      (`KismetSystemLibrary.PrintText` "Вы нажали кнопку 2"))
    (:`2`
      (`KismetSystemLibrary.PrintText` "Вы нажали кнопку 3")))
  (`self.RestorePlayerInput`)
  (set `self.DialogueUIRef` null))

(fn `Create Dialog Widget`
  (bind _returnvalue (`GameplayStatics.GetPlayerController` 0))
  (bind _pressetodialogueref (`self.PressEToDialogueRef`))
  (if (`KismetSystemLibrary.IsValid` _pressetodialogueref)
    (`Widget.RemoveFromParent` _pressetodialogueref))
  (bind _returnvalue_2 (`|CreateWidget` "/Game/UI/Dialogs/WBP_Dialogue_Anubis.WBP_Dialogue_Anubis_C"))
  (`UserWidget.AddToViewport` _returnvalue_2 0)
  (set `self.DialogueUIRef` _returnvalue_2)
  (set `TextBlock.Text` "Привет! Это Анубис, хехе)))" (`/Game/UI/Dialogs/WBP_Dialogue_Anubis.SubtitleText_Anubis` (`self.DialogueUIRef`)))
  (bind _asbp_third_person_character (cast `/Game/ThirdPerson/Blueprints/BP_Player` (`GameplayStatics.GetPlayerCharacter` 0)))
  (set `/Game/ThirdPerson/Blueprints/BP_Player.CurrentNPC` self _asbp_third_person_character)
  (`WidgetBlueprintLibrary.SetInputMode_GameAndUIEx` _returnvalue _returnvalue_2 "DoNotLock" false)
  (set `PlayerController.bShowMouseCursor` false _returnvalue))

(fn `PlayTalkingAnimMontage`)

(fn `RestorePlayerInput`
  (bind _returnvalue (`GameplayStatics.GetPlayerController` 0))
  (`WidgetBlueprintLibrary.SetInputMode_GameOnly` _returnvalue)
  (set `PlayerController.bShowMouseCursor` false _returnvalue))

(fn `RotateToPlayer`
  (`self.K2_SetActorRotation` (`KismetMathLibrary.FindLookAtRotation` (`self.K2_GetActorLocation`) (`self.K2_GetActorLocation` (`GameplayStatics.GetPlayerCharacter` 0)))))

(fn `UserConstructionScript`)