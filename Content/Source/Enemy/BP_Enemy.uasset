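; Melee enemy character that detects the player, chases, attacks, and dies when health runs out.
; Detection and attack spheres set state that Tick reads to face the player, run AIMoveTo, or call StartAttackLoop each frame.
; The looping timer and CanAttack-gated montage drive attacks, while a separate EnemyAttack function applies damage.
; AnyDamage updates the health bar widget and plays the death montage at zero health.
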(event `self.ReceiveTick`
  (params (DeltaSeconds :type "Float (single-precision)"))
  (bind _charactermovement (`self.CharacterMovement`))
  (if (`self.IsInDetectionRange`)
    (`self.RotateToPlayer`)
    (if (`self.IsInAttackRange`)
      (`MovementComponent.StopMovementImmediately` _charactermovement)
      (`self.StartAttackLoop`)
      (else
        (bind _asbp_melee_aicontroller (cast `/Game/Source/AI/BP_MeleeAIController` (`self.GetController`)))
        (bind _isanimplaying (`self.CheckIfAnimPlaying`))
        (if (not _isanimplaying)
          (`|AIMoveTo` _asbp_melee_aicontroller self (0.0 0.0 0.0) (`self.TargetPlayer`) 120.0))))
    (else
      (`MovementComponent.StopMovementImmediately` _charactermovement))))

(event `self.ReceiveBeginPlay`
  (bind _aswbm_enemy_hb (cast `/Game/UI/Common/WBM_ENEMY_HB` (`WidgetComponent.GetUserWidgetObject` (`self.HealthBarWidget`))))
  (bind _output_get (set `self.As WBM ENEMY HB` _aswbm_enemy_hb)))

(event `self.DetectionRadius.OnComponentBeginOverlap`
  (params (OverlappedComponent :type "PrimitiveComponent Object Reference") (OtherActor :type "Actor Object Reference") (OtherComp :type "PrimitiveComponent Object Reference") (OtherBodyIndex :type Integer) (bFromSweep :type Boolean) (SweepResult :type "HitResult Structure (by ref)"))
  (bind _asbp_player (cast `/Game/ThirdPerson/Blueprints/BP_Player` OtherActor))
  (set `self.TargetPlayer` _asbp_player)
  (set `self.IsInDetectionRange` true)
  (set `self.CanAttack` true))

(event `self.AttackRadius.OnComponentBeginOverlap`
  (params (OverlappedComponent :type "PrimitiveComponent Object Reference") (OtherActor :type "Actor Object Reference") (OtherComp :type "PrimitiveComponent Object Reference") (OtherBodyIndex :type Integer) (bFromSweep :type Boolean) (SweepResult :type "HitResult Structure (by ref)"))
  (cast `/Game/ThirdPerson/Blueprints/BP_Player` OtherActor)
  (set `self.IsInAttackRange` true))

(event `self.AttackRadius.OnComponentEndOverlap`
  (params (OverlappedComponent :type "PrimitiveComponent Object Reference") (OtherActor :type "Actor Object Reference") (OtherComp :type "PrimitiveComponent Object Reference") (OtherBodyIndex :type Integer))
  (cast `/Game/ThirdPerson/Blueprints/BP_Player` OtherActor)
  (set `self.IsInAttackRange` false)
  (`KismetSystemLibrary.K2_ClearAndInvalidateTimerHandle` (`self.AttackTimerHandle`)))

(event `self.DetectionRadius.OnComponentEndOverlap`
  (params (OverlappedComponent :type "PrimitiveComponent Object Reference") (OtherActor :type "Actor Object Reference") (OtherComp :type "PrimitiveComponent Object Reference") (OtherBodyIndex :type Integer))
  (cast `/Game/ThirdPerson/Blueprints/BP_Player` OtherActor)
  (set `self.TargetPlayer` null)
  (`KismetSystemLibrary.K2_ClearAndInvalidateTimerHandle` (`self.AttackTimerHandle`))
  (set `self.IsInDetectionRange` false)
  (set `self.CanAttack` false))

(event `self.ReceiveAnyDamage`
  (params (Damage :type "Float (single-precision)") (DamageType :type "DamageType Object Reference") (InstigatedBy :type "Controller Object Reference") (DamageCauser :type "Actor Object Reference"))
  (if (not (`self.IsDead`))
    (`KismetSystemLibrary.PrintText` "Hello")
    (bind _output_get (set `self.Health` (- (`self.Health`) Damage)))
    (set `/Game/UI/Common/WBM_ENEMY_HB.Health` (/ _output_get (`self.MaxHealth`)) (`self.As WBM ENEMY HB`))
    (if (<= _output_get 0.0)
      (set `self.IsDead` true)
      (`MovementComponent.StopMovementImmediately` (`self.CharacterMovement`))
      (`self.PlayAnimMontage` (`.DeathMontage_2_A2D8E61C44BFF87BC4F99793AD41A60F` (break `/Game/Source/Enemy/S_EnemyAnimations` (`self.Animations`))))
      (else
        (`KismetSystemLibrary.PrintText` (`KismetTextLibrary.Conv_DoubleToText` Damage "HalfToEven"))))))

(event `Perform Attack`
  (`self.PerformAttackFunc`))

(fn `CheckIfAnimPlaying`
  (returns (isAnimPlaying :type Boolean))
  (bind (_deathmontage _attackmontage) (break `/Game/Source/Enemy/S_EnemyAnimations` (`self.Animations`)))
  (bind _returnvalue (`SkeletalMeshComponent.GetAnimInstance` (`self.Mesh`)))
  (if (or (`AnimInstance.Montage_IsPlaying` _returnvalue _attackmontage) (`AnimInstance.Montage_IsPlaying` _returnvalue _deathmontage))
    (return true)
    (else
      (return false))))

(fn `EnemyAttack`
  (bind _targetplayer (`self.TargetPlayer`))
  (if (`self.IsInAttackRange`)
    (`/Engine/EditorBlueprintResources/StandardMacros.IsValid` _targetplayer
      (:`Is Valid`
        (`GameplayStatics.ApplyDamage` _targetplayer (`self.AttackDamage`) null self)))))

(fn `PerformAttackFunc`
  (bind _targetplayer (`self.TargetPlayer`))
  (if (and (`self.IsInAttackRange`) (`KismetSystemLibrary.IsValid` _targetplayer) (!= (`/Game/ThirdPerson/Blueprints/BP_Player.IsDead` _targetplayer) true) (`self.CanAttack`))
    (`MovementComponent.StopMovementImmediately` (`self.CharacterMovement`))
    (set `self.CanAttack` false)
    (`self.PlayAttackMontage`)))

(fn `PlayAttackMontage`
  (`self.PlayAnimMontage` (`.AttackMontage_4_06F6015C47DDA3DB83870AB8747FF501` (break `/Game/Source/Enemy/S_EnemyAnimations` (`self.Animations`)))))

(fn `RotateToPlayer`
  (`self.K2_SetActorRotation` (`KismetMathLibrary.FindLookAtRotation` (`self.K2_GetActorLocation`) (`self.K2_GetActorLocation` (`GameplayStatics.GetPlayerCharacter` 0)))))

(fn `StartAttackLoop`
  (if (`self.IsInAttackRange`)
    (`self.Perform Attack`)
    (bind _returnvalue (`KismetSystemLibrary.K2_SetTimerDelegate` (`|CreateDelegate` :!event `Perform Attack`) (`self.AttackInterval`) true))
    (set `self.AttackTimerHandle` _returnvalue)))

(fn `UserConstructionScript`)