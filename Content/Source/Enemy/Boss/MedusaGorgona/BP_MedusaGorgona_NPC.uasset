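; Medusa Gorgon boss NPC that opens a riddle dialogue and can turn into the hostile boss.
; It extends a parent NPC's talk montage and dialog creation, choosing the widget by the player's skin type.
; The "smart" skin gets a three-answer riddle flagged as boss dialogue, while others get a dismissive line and StartAttack.
; StartAttack waits briefly, spawns BP_MedusaGorgona at the NPC's transform and destroys the NPC.
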(event `StartAttack`
  (`KismetSystemLibrary.Delay` 2.0)
  (`KismetSystemLibrary.PrintText` "ГОРОГОНА НАПАДАЕТ")
  (`|SpawnActorFromClass` "/Game/Source/Enemy/Boss/MedusaGorgona/BP_MedusaGorgona.BP_MedusaGorgona_C" (`self.GetTransform`) "Undefined" "MultiplyWithRoot" null null)
  (`self.K2_DestroyActor`))

(fn `CheckThatPlayerIsSmart`
  (returns (IsSmart :type Boolean))
  (bind _asbp_player (cast `/Game/ThirdPerson/Blueprints/BP_Player` (`GameplayStatics.GetPlayerCharacter` 0)))
  (return (`|EnumEquality` (`/Game/ThirdPerson/Blueprints/BP_Player.PlayerSkinType` _asbp_player) "NewEnumerator0")))

(fn `Create Dialog Widget`
  (bind _returnvalue (`GameplayStatics.GetPlayerController` 0))
  (`parent.Create Dialog Widget`)
  (bind _issmart (`self.CheckThatPlayerIsSmart`))
  (if _issmart
    (bind _returnvalue_2 (`|CreateWidget` "/Game/UI/Dialogues/WBP_Dialogue_3Variants.WBP_Dialogue_3Variants_C"))
    (set `/Game/UI/Dialogues/WBP_Dialogue_3Variants.IsBossDialogue` true _returnvalue_2)
    (`UserWidget.AddToViewport` _returnvalue_2 0)
    (bind _output_get (set `self.DialogueUIRef` _returnvalue_2))
    (bind _aswbp_dialogue_3variants (cast `/Game/UI/Dialogues/WBP_Dialogue_3Variants` _output_get))
    (set `TextBlock.Text` "ГОРГОНА:" (`/Game/UI/Dialogues/WBP_Dialogue_3Variants.FraseAuthor` _aswbp_dialogue_3variants))
    (set `TextBlock.Text` "Отгадай мою загадку: " (`/Game/UI/Dialogues/WBP_Dialogue_3Variants.SubtitleText` _aswbp_dialogue_3variants))
    (`self.SetQuestionVariants`)
    (`WidgetBlueprintLibrary.SetInputMode_UIOnlyEx` _returnvalue _output_get)
    (set `PlayerController.bShowMouseCursor` false _returnvalue)
    (else
      (bind _returnvalue_3 (`|CreateWidget` "/Game/UI/Dialogues/WBP_Dialogue_0Variants.WBP_Dialogue_0Variants_C"))
      (`UserWidget.AddToViewport` _returnvalue_3 0)
      (bind _output_get_2 (set `self.DialogueUIRef` _returnvalue_3))
      (bind _aswbp_dialogue_0variants (cast `/Game/UI/Dialogues/WBP_Dialogue_0Variants` _output_get_2))
      (set `TextBlock.Text` "ГОРГОНА:" (`/Game/UI/Dialogues/WBP_Dialogue_0Variants.FraseAuthor` _aswbp_dialogue_0variants))
      (set `TextBlock.Text` "Ты недостаточно умный чтобы угадывать мои загадки" (`/Game/UI/Dialogues/WBP_Dialogue_0Variants.SubtitleText` _aswbp_dialogue_0variants))
      (`self.StartAttack`))))

(fn `PlayTalkingAnimMontage`
  (`parent.PlayTalkingAnimMontage`)
  (`self.PlayAnimMontage` "/Game/Source/Enemy/Boss/MedusaGorgona/Animations/AM_MedusaGorgona_NPCSawPlayer.AM_MedusaGorgona_NPCSawPlayer"))

(fn `SetQuestionVariants`
  (bind _aswbp_dialogue_3variants (cast `/Game/UI/Dialogues/WBP_Dialogue_3Variants` (`self.DialogueUIRef`)))
  (set `TextBlock.Text` "Пупа" (`/Game/UI/Dialogues/WBP_Dialogue_3Variants.ResponseText1` _aswbp_dialogue_3variants))
  (set `TextBlock.Text` "Лупа" (`/Game/UI/Dialogues/WBP_Dialogue_3Variants.ResponseText2` _aswbp_dialogue_3variants))
  (set `TextBlock.Text` "Лампочка" (`/Game/UI/Dialogues/WBP_Dialogue_3Variants.ResponseText3` _aswbp_dialogue_3variants)))

(fn `UserConstructionScript`
  (`parent.UserConstructionScript`))