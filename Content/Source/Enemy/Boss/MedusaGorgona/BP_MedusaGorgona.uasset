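; Medusa Gorgona boss enemy Blueprint that extends a parent enemy class with its own death and attack montages.
; An overlap radius tracks whether the player is in melee reach, choosing the melee montage up close or randomly earth slam or lightning otherwise.
; Attacks start only on a valid living target in range, stopping movement first.
; Each attack function sets its damage type before running the parent attack.
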(event `self.ReceiveBeginPlay`
  (`parent.ReceiveBeginPlay`)
  (set `self.Animations` (make `/Game/Source/Enemy/S_EnemyAnimations` "/Game/Source/Enemy/Boss/MedusaGorgona/Animations/AM_MedusaGorgona_FallingDown.AM_MedusaGorgona_FallingDown" "/Game/Source/Enemy/Boss/MedusaGorgona/Animations/AM_MedusaGorgona_MeleeAttack.AM_MedusaGorgona_MeleeAttack"))
  (set `self.EnemyDamageType` "NewEnumerator0"))

(event `self.MeleeAttackRadius.OnComponentBeginOverlap`
  (params (OverlappedComponent :type "PrimitiveComponent Object Reference") (OtherActor :type "Actor Object Reference") (OtherComp :type "PrimitiveComponent Object Reference") (OtherBodyIndex :type Integer) (bFromSweep :type Boolean) (SweepResult :type "HitResult Structure (by ref)"))
  (cast `/Game/ThirdPerson/Blueprints/BP_Player` OtherActor)
  (set `self.IsInMeleeRadius` true))

(event `self.MeleeAttackRadius.OnComponentEndOverlap`
  (params (OverlappedComponent :type "PrimitiveComponent Object Reference") (OtherActor :type "Actor Object Reference") (OtherComp :type "PrimitiveComponent Object Reference") (OtherBodyIndex :type Integer))
  (cast `/Game/ThirdPerson/Blueprints/BP_Player` OtherActor)
  (set `self.IsInMeleeRadius` false))

(fn `CheckIfAnimPlaying`
  (returns (isAnimPlaying :type Boolean))
  (bind _returnvalue (`SkeletalMeshComponent.GetAnimInstance` (`self.Mesh`)))
  (if (or (`AnimInstance.Montage_IsPlaying` _returnvalue "/Game/Source/Enemy/Boss/MedusaGorgona/Animations/AM_MedusaGorgona_FallingDown.AM_MedusaGorgona_FallingDown") (`AnimInstance.Montage_IsPlaying` _returnvalue "/Game/Source/Enemy/Boss/MedusaGorgona/Animations/AM_MedusaGorgona_EarthSlamAttack.AM_MedusaGorgona_EarthSlamAttack") (`AnimInstance.Montage_IsPlaying` _returnvalue "/Game/Source/Enemy/Boss/MedusaGorgona/Animations/AM_MedusaGorgona_LightningAttack.AM_MedusaGorgona_LightningAttack") (`AnimInstance.Montage_IsPlaying` _returnvalue "/Game/Source/Enemy/Boss/MedusaGorgona/Animations/AM_MedusaGorgona_MeleeAttack.AM_MedusaGorgona_MeleeAttack"))
    (return true)
    (else
      (return false))))

(fn `EarthSlamAttack`
  (set `self.EnemyDamageType` "NewEnumerator1")
  (`parent.EnemyAttack`))

(fn `LightningAttack`
  (set `self.EnemyDamageType` "NewEnumerator3")
  (`parent.EnemyAttack`))

(fn `MeleeAttack`
  (set `self.EnemyDamageType` "NewEnumerator0")
  (`parent.EnemyAttack`))

(fn `PerformAttackFunc`
  (bind _targetplayer (`self.TargetPlayer`))
  (if (and (`self.IsInAttackRange`) (`KismetSystemLibrary.IsValid` _targetplayer) (!= (`/Game/ThirdPerson/Blueprints/BP_Player.IsDead` _targetplayer) true) (`self.CanAttack`))
    (`MovementComponent.StopMovementImmediately` (`self.CharacterMovement`))
    (set `self.CanAttack` false)
    (`self.PlayAttackMontage`)))

(fn `PlayAttackMontage`
  (if (`self.IsInMeleeRadius`)
    (`self.PlayAnimMontage` "/Game/Source/Enemy/Boss/MedusaGorgona/Animations/AM_MedusaGorgona_MeleeAttack.AM_MedusaGorgona_MeleeAttack")
    (else
      (switch `int` (`KismetMathLibrary.RandomIntegerInRange` 0 1)
        (:`0`
          (`self.PlayAnimMontage` "/Game/Source/Enemy/Boss/MedusaGorgona/Animations/AM_MedusaGorgona_EarthSlamAttack.AM_MedusaGorgona_EarthSlamAttack"))
        (:`1`
          (`self.PlayAnimMontage` "/Game/Source/Enemy/Boss/MedusaGorgona/Animations/AM_MedusaGorgona_LightningAttack.AM_MedusaGorgona_LightningAttack"))))))

(fn `UserConstructionScript`
  (`parent.UserConstructionScript`))