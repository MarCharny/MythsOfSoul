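; Greek Enchantress ranged enemy, a child Blueprint that attacks by spawning fireballs.
; BeginPlay runs the parent logic, then sets the death and ranged attack montages and the enemy damage type.
; EnemyAttack calls SpawnFireball, which spawns a BP_Fireball owned by the enemy at the mesh's FireballSpawn socket location and stores the reference.
; The spawn uses only the socket's location, not its rotation.
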(event `self.ReceiveBeginPlay`
  (`parent.ReceiveBeginPlay`)
  (set `self.Animations` (make `/Game/Source/Enemy/S_EnemyAnimations` "/Game/Source/Enemy/Ranged/GreekEnchantress/Animations/AM_GreekEnchantress_Death.AM_GreekEnchantress_Death" "/Game/Source/Enemy/Ranged/GreekEnchantress/Animations/AM_GreekEnchantress_RangedAttack.AM_GreekEnchantress_RangedAttack"))
  (set `self.EnemyDamageType` "NewEnumerator2"))

(fn `EnemyAttack`
  (`self.SpawnFireball`))

(fn `SpawnFireball`
  (bind _returnvalue (`|SpawnActorFromClass` "/Game/Source/Enemy/Ranged/Fireball/BP_Fireball.BP_Fireball_C" (`KismetMathLibrary.Conv_VectorToTransform` (`SceneComponent.GetSocketLocation` (`self.Mesh`) "FireballSpawn")) "Undefined" "MultiplyWithRoot" self null))
  (set `self.SpawnedFireball` _returnvalue))

(fn `UserConstructionScript`
  (`parent.UserConstructionScript`))