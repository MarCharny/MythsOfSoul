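; BP_Fireball is a projectile, filed under ranged enemies, that launches toward player 0 and deals damage on overlap.
; At BeginPlay it computes a look-at direction to the player once and passes it, scaled by FireballSpeed, to SetVelocityInLocalSpace, despite being a world-space vector.
; Collision overlaps with BP_Enemy only print debug text.
; Any other non-owner actor receives FireballDamage, triggers debug text and destroys the fireball.
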(event `self.ReceiveBeginPlay`
  (`ProjectileMovementComponent.SetVelocityInLocalSpace` (`self.ProjectileMovement`) (* (`KismetMathLibrary.GetForwardVector` (`KismetMathLibrary.FindLookAtRotation` (`self.K2_GetActorLocation` self) (`self.K2_GetActorLocation` (`GameplayStatics.GetPlayerCharacter` 0)))) (`self.FireballSpeed`))))

(event `self.Collision.OnComponentBeginOverlap`
  (params (OverlappedComponent :type "PrimitiveComponent Object Reference") (OtherActor :type "Actor Object Reference") (OtherComp :type "PrimitiveComponent Object Reference") (OtherBodyIndex :type Integer) (bFromSweep :type Boolean) (SweepResult :type "HitResult Structure (by ref)"))
  (cast `/Game/Source/Enemy/BP_Enemy` OtherActor
    (:`then`
      (`KismetSystemLibrary.PrintText` "ENEMYYYY"))
    (:`CastFailed`
      (if (!= OtherActor (`self.GetOwner`))
        (`GameplayStatics.ApplyDamage` OtherActor (`self.FireballDamage`) null self)
        (`KismetSystemLibrary.PrintText` "ПОПАЛ!")
        (`self.K2_DestroyActor`)))))

(fn `UserConstructionScript`)