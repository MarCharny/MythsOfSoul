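; BP_MeleeEnemy is a melee AI enemy that chases the player, attacks up close and is destroyed when its health runs out.
; A detection overlap starts AIMoveTo through BP_MeleeAIController, and an attack-range overlap plays a montage and starts a looping timer.
; CanAttack gates the montage and resets only on re-detection; EnemyAttack applies damage but is not called here.
; Incoming damage updates a health bar widget.
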(event `self.ReceiveBeginPlay`
  (bind _aswbm_enemy_hb (cast `/Game/UI/Common/WBM_ENEMY_HB` (`WidgetComponent.GetUserWidgetObject` (`self.HealthBarWidget`))))
  (bind _output_get (set `self.As WBM ENEMY HB` _aswbm_enemy_hb)))

(event `self.DetectionRadius.OnComponentBeginOverlap`
  (params (OverlappedComponent :type "PrimitiveComponent Object Reference") (OtherActor :type "Actor Object Reference") (OtherComp :type "PrimitiveComponent Object Reference") (OtherBodyIndex :type Integer) (bFromSweep :type Boolean) (SweepResult :type "HitResult Structure (by ref)"))
  (bind _asbp_third_person_character (cast `/Game/ThirdPerson/Blueprints/BP_ThirdPersonCharacter` OtherActor))
  (set `self.TargetPlayer` _asbp_third_person_character)
  (set `self.CanAttack` true)
  (bind _asbp_melee_aicontroller (cast `/Game/Source/AI/BP_MeleeAIController` (`self.GetController`))
    (:`then`
      (`|AIMoveTo` _asbp_melee_aicontroller self (0.0 0.0 0.0) (`self.TargetPlayer`) 120.0))
    (:`CastFailed`
      (`KismetSystemLibrary.PrintText` "Hello"))))

(event `self.AttackRadius.OnComponentBeginOverlap`
  (params (OverlappedComponent :type "PrimitiveComponent Object Reference") (OtherActor :type "Actor Object Reference") (OtherComp :type "PrimitiveComponent Object Reference") (OtherBodyIndex :type Integer) (bFromSweep :type Boolean) (SweepResult :type "HitResult Structure (by ref)"))
  (cast `/Game/ThirdPerson/Blueprints/BP_ThirdPersonCharacter` OtherActor)
  (set `self.IsInAttackRange` true)
  (`self.StartAttackLoop`))

(event `self.AttackRadius.OnComponentEndOverlap`
  (params (OverlappedComponent :type "PrimitiveComponent Object Reference") (OtherActor :type "Actor Object Reference") (OtherComp :type "PrimitiveComponent Object Reference") (OtherBodyIndex :type Integer))
  (cast `/Game/ThirdPerson/Blueprints/BP_ThirdPersonCharacter` OtherActor)
  (set `self.IsInAttackRange` false)
  (`KismetSystemLibrary.K2_ClearAndInvalidateTimerHandle` (`self.AttackTimerHandle`))
  (`|AIMoveTo` self (0.0 0.0 0.0) (`self.TargetPlayer`) 80.0))

(event `self.DetectionRadius.OnComponentEndOverlap`
  (params (OverlappedComponent :type "PrimitiveComponent Object Reference") (OtherActor :type "Actor Object Reference") (OtherComp :type "PrimitiveComponent Object Reference") (OtherBodyIndex :type Integer))
  (cast `/Game/ThirdPerson/Blueprints/BP_ThirdPersonCharacter` OtherActor)
  (set `self.TargetPlayer` null)
  (`KismetSystemLibrary.K2_ClearAndInvalidateTimerHandle` (`self.AttackTimerHandle`))
  (`MovementComponent.StopMovementImmediately` (`self.CharacterMovement`)))

(event `self.ReceiveAnyDamage`
  (params (Damage :type "Float (single-precision)") (DamageType :type "DamageType Object Reference") (InstigatedBy :type "Controller Object Reference") (DamageCauser :type "Actor Object Reference"))
  (`KismetSystemLibrary.PrintText` "Hello")
  (bind _output_get (set `self.Health` (- (`self.Health`) Damage)))
  (set `/Game/UI/Common/WBM_ENEMY_HB.Health` (/ _output_get (`self.MaxHealth`)) (`self.As WBM ENEMY HB`))
  (if (<= _output_get 0.0)
    (`self.K2_DestroyActor`)
    (`KismetSystemLibrary.PrintText` "actor destroyed")
    (else
      (`KismetSystemLibrary.PrintText` (`KismetTextLibrary.Conv_DoubleToText` Damage "HalfToEven")))))

(event `Perform Attack`
  (if (and (`self.IsInAttackRange`) (`KismetSystemLibrary.IsValid` (`self.TargetPlayer`)) (`self.CanAttack`))
    (`MovementComponent.StopMovementImmediately` (`self.CharacterMovement`))
    (set `self.CanAttack` false)
    (`self.PlayAnimMontage` "/Game/Source/Enemy/MM_Attack_02_Montage.MM_Attack_02_Montage")))

(fn `EnemyAttack`
  (bind _targetplayer (`self.TargetPlayer`))
  (`/Engine/EditorBlueprintResources/StandardMacros.IsValid` _targetplayer
    (:`Is Valid`
      (`GameplayStatics.ApplyDamage` _targetplayer (`self.AttackDamage`)))))

(fn `StartAttackLoop`
  (if (`self.IsInAttackRange`)
    (`KismetSystemLibrary.PrintText` "Play anim atack montage")
    (`self.Perform Attack`)
    (bind _returnvalue (`KismetSystemLibrary.K2_SetTimerDelegate` (`|CreateDelegate` :!event `Perform Attack`) (`self.AttackInterval`) true))
    (set `self.AttackTimerHandle` _returnvalue)))

(fn `UserConstructionScript`)