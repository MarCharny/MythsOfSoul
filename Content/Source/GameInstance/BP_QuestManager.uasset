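; BP_QuestManager manages main and side quest progression, built on a Quests DataTable and a per-quest state map.
; Init restores saved state or seeds the map from the table, then tries to start the initial quest.
; Step completion acts on the tracked quest and leads into CompleteQuest, which updates dependent quests, chains main quests or retracks the main one after side quests.
; Rewards are only a debug-print stub, and several lookups pass None IDs.
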(fn `CanStartQuest`
  (params (QuestId :type Name))
  (returns (CanStart :type Boolean))
  (`KismetSystemLibrary.PrintText` null "Entered CanStartQuest" true true (struct :`R` 1.0 :`B` 0.616252 :`A` 1.0) 10.0)
  (if (`KismetArrayLibrary.Array_Contains` (`self.CompletedQuests`) QuestId)
    (return false)
    (else
      (bind (_found _questdata) (`self.GetQuestData` "None"))
      (if _found
        (return (`KismetArrayLibrary.Array_Contains` (`self.CompletedQuests`) (`.RequiredMainId_26_0452890D49B727BCA8FC8CA279E260FE` (break `/Game/Source/QuestSystem/S_QuestData` _questdata))))
        (else
          (return false))))))

(fn `CompleteQuest`
  (params (QuestId :type Name))
  (`KismetSystemLibrary.PrintText` null "Entered CompleteQuest" true true (struct :`R` 1.0 :`G` 0.002983 :`B` 0.528071 :`A` 1.0))
  (bind (_found _questdata) (`self.GetQuestData` QuestId))
  (bind (_questid _title _description _questtype _rewardsartifacts _rewardspotions _requiredmainid _steps _startlocation _startlocationrad _nextmainquestid) (break `/Game/Source/QuestSystem/S_QuestData` _questdata))
  (`self.GiveRewards` _rewardspotions _rewardsartifacts)
  (bind _structout (setmembers `/Game/Source/QuestSystem/S_QuestState` :`StructRef` (`BlueprintMapLibrary.Map_Find` (`self.QuestsState`) QuestId) :`Status` "NewEnumerator2" :`CurrentStepStatus` "NewEnumerator2"))
  (`BlueprintMapLibrary.Map_Add` (`self.QuestsState`) QuestId _structout)
  (`KismetArrayLibrary.Array_Add` (`self.CompletedQuests`) QuestId)
  (`self.SetAvaliabilityForQuests` QuestId)
  (switch `/Game/Source/QuestSystem/E_QuestType` _questtype
    (:`NewEnumerator0`
      (`self.StartQuest` _nextmainquestid)
      (`KismetSystemLibrary.PrintText` null "Completed Main Quest" true true (struct :`G` 1.0 :`B` 0.012274 :`A` 1.0))
      (`GameplayStatics.SaveGameToSlot` null))
    (:`NewEnumerator1`
      (`self.SetTrackedQuest` (`self.CurrentMainQuest`))
      (`KismetSystemLibrary.PrintText` null "Completed side quest!" true true (struct :`G` 1.0 :`B` 0.039209 :`A` 1.0)))))

(fn `CompleteStep`
  (params (QuestId :type Name) (StedId :type Integer))
  (returns (Succsess :type Boolean))
  (if (== QuestId (`self.TrackedQuestId`))
    (if true
      (switch `/Game/Source/QuestSystem/E_QuestStepStatus` (`.CurrentStepStatus_12_EABFD94044B94B7B64D896BDBBBF52A9` (break `/Game/Source/QuestSystem/S_QuestState` (`BlueprintMapLibrary.Map_Find` (`self.QuestsState`) QuestId)))
        (:`NewEnumerator0`
          (return false))
        (:`NewEnumerator1`
          (bind _success (`self.StartNextStep` QuestId StedId))
          (if _success
            (return false)
            (else
              (return false))))
        (:`NewEnumerator2`
          (return false))))
    (else
      (return false))))

(fn `GetQuestData`
  (params (QuestId :type Name))
  (returns (Found :type Boolean) (QuestData :type "/Game/Source/QuestSystem/S_QuestData Structure"))
  (bind _returnvalue (`|GetDataTableRow` (`self.Quests`) QuestId)
    (:`then`
      (return true _returnvalue))
    (:`RowNotFound`
      (return false))))

(fn `GiveRewards`
  (params (PotionsReward :type "Array of /Game/Source/QuestSystem/S_PotionReward Structure") (ArtifactsReward :type "Array of /Game/Source/Inventory/S_ArtifactInstance Structure"))
  (`KismetSystemLibrary.PrintText` null "TRY TO GIVE REWARDS" true true (struct :`R` 0.931697 :`G` 1.0 :`B` 0.927776 :`A` 1.0)))

(fn `Init`
  (params (FromSave :type Boolean) (QuestsStates :type "Map of Name to /Game/Source/QuestSystem/S_QuestState Structure") (TrackedId :type Name) (CurrentMainQuest :type Name))
  (bind _quests (`self.Quests`))
  (bind _questsstate (`self.QuestsState`))
  (bind _start_quest (`self.Start Quest`))
  (`KismetSystemLibrary.PrintText` null "INIT QUEST SYSTEM" true true (struct :`G` 1.0 :`B` 0.789899 :`A` 1.0) 30.0)
  (if FromSave
    (set `self.TrackedQuestId` TrackedId)
    (set `self.CurrentMainQuest` "None")
    (set `self.QuestsState` QuestsStates)
    (`KismetSystemLibrary.PrintText` null "Loaded quests from Save" true true (struct :`G` 1.0 :`B` 0.012274 :`A` 1.0) 10.0)
    (else
      (bind _outrownames (`DataTableFunctionLibrary.GetDataTableRowNames` _quests))
      (for _array_element _outrownames
        (bind _returnvalue (`|GetDataTableRow` _quests _array_element)
          (:`then`
            (bind _questid (break `/Game/Source/QuestSystem/S_QuestData` _returnvalue))
            (if (== _start_quest _questid)
              (`BlueprintMapLibrary.Map_Add` _questsstate _questid (make `/Game/Source/QuestSystem/S_QuestState` "NewEnumerator1" 0 "NewEnumerator1"))
              (else
                (`BlueprintMapLibrary.Map_Add` _questsstate _questid (make `/Game/Source/QuestSystem/S_QuestState` "NewEnumerator4" 0 "NewEnumerator1")))))))
      (bind _successed (`self.StartQuest` _start_quest))
      (if _successed
        (`KismetSystemLibrary.PrintText` null "STARTED QUEST" true true (struct :`G` 1.0 :`B` 0.19539 :`A` 1.0) 10.0)
        (else
          (`KismetSystemLibrary.PrintText` null "FAILED TO START INIT QUEST" true true (struct :`G` 1.0 :`B` 0.012274 :`A` 1.0) 10.0))))))

(fn `SetAvaliabilityForQuests`
  (params (CompletedQuestId :type Name))
  (bind _quests (`self.Quests`))
  (bind _outrownames (`DataTableFunctionLibrary.GetDataTableRowNames` _quests))
  (for _array_element _outrownames
    (bind _returnvalue (`|GetDataTableRow` _quests _array_element)
      (:`then`
        (bind (_questid _title _description _questtype _rewardsartifacts _rewardspotions _requiredmainid) (break `/Game/Source/QuestSystem/S_QuestData` _returnvalue))
        (if (== CompletedQuestId _requiredmainid)
          (setmembers `/Game/Source/QuestSystem/S_QuestState` :`StructRef` (`BlueprintMapLibrary.Map_Find` (`self.QuestsState`) _questid) :`Status` "NewEnumerator3")))))
  (return))

(fn `SetTrackedQuest`
  (params (QuestId :type Name))
  (`KismetSystemLibrary.PrintText` null "Enterted SetTrackedQuest" true true (struct :`R` 1.0 :`G` 0.028795 :`B` 0.713967 :`A` 1.0))
  (if (`.ReturnValue` (`BlueprintMapLibrary.Map_Find` (`self.QuestsState`) QuestId))
    (set `self.TrackedQuestId` QuestId)
    (return)
    (else
      (return))))

(fn `StartNextStep`
  (params (QuestId :type Name) (StepId :type Integer))
  (returns (Success :type Boolean))
  (locals (QuestTable :type "DataTable Object Reference" :default "/Script/Engine.DataTable'/Game/Source/QuestSystem/DT_Quests.DT_Quests'") (QuestStates :type "Map of Name to /Game/Source/QuestSystem/S_QuestState Structure") (TrackedQuest :type Name) (CompledetQuests :type "Array of Name"))
  (bind (_value _returnvalue) (`BlueprintMapLibrary.Map_Find` (`local.QuestStates`) QuestId))
  (if (== QuestId (`self.TrackedQuestId`))
    (bind (_found _questdata) (`self.GetQuestData` "None"))
    (if _found
      (if (>= StepId (`KismetArrayLibrary.Array_Length` (`.Steps_32_51BC1AE446C56A77A68E48AADD133128` (break `/Game/Source/QuestSystem/S_QuestData` _questdata))))
        (`self.CompleteQuest` "None")
        (elif _returnvalue
          (bind _structout (setmembers `/Game/Source/QuestSystem/S_QuestState` :`StructRef` _value :`Status` "NewEnumerator1" :`CurrentStepId` StepId))
          (`BlueprintMapLibrary.Map_Add` (`self.QuestsState`) QuestId _structout)
          (return true)
          (else
            (return false))))
      (else
        (return false)))
    (else
      (return false))))

(fn `StartQuest`
  (params (QuestId :type Name))
  (returns (Successed :type Boolean))
  (bind (_value _returnvalue) (`BlueprintMapLibrary.Map_Find` (`self.QuestsState`) QuestId))
  (`KismetSystemLibrary.PrintText` null "START QUEST" true true (struct :`R` 1.0 :`G` 0.996182 :`B` 0.894848 :`A` 1.0) 10.0)
  (bind _canstart (`self.CanStartQuest` QuestId))
  (if _canstart
    (if _returnvalue
      (bind _structout (setmembers `/Game/Source/QuestSystem/S_QuestState` :`StructRef` _value :`Status` "NewEnumerator1" :`CurrentStepId` 0 :`CurrentStepStatus` "NewEnumerator1"))
      (`BlueprintMapLibrary.Map_Add` (`self.QuestsState`) QuestId _structout)
      (`self.SetTrackedQuest` QuestId)
      (bind (_found _questdata) (`self.GetQuestData` QuestId))
      (switch `/Game/Source/QuestSystem/E_QuestType` (`.QuestType_11_52F6F8DE4F4A13258E9661989F8AE8C3` (break `/Game/Source/QuestSystem/S_QuestData` _questdata))
        (:`NewEnumerator0`
          (set `self.CurrentMainQuest` "None")
          (return true))
        (:`NewEnumerator1`
          (return true)))
      (else
        (return false)))
    (else
      (return false))))