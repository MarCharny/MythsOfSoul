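; BP_QuestStartTrigger is a trigger actor that starts a quest or completes a quest step when the player enters its sphere.
; On overlap it casts to BP_Player and calls that player's QuestManagmentSystem: StartQuest for step zero, CompleteStep for any other StepId.
; Success sets WasTriggered, which blocks later activations only when DisableAfterStart is set.
; Debug prints trace the overlap, cast and failures.
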(event `self.QuestStartSphere.OnComponentBeginOverlap`
  (params (OverlappedComponent :type "PrimitiveComponent Object Reference") (OtherActor :type "Actor Object Reference") (OtherComp :type "PrimitiveComponent Object Reference") (OtherBodyIndex :type Integer) (bFromSweep :type Boolean) (SweepResult :type "HitResult Structure (by ref)"))
  (bind _stepid (`self.StepId`))
  (bind _questid (`self.QuestId`))
  (`KismetSystemLibrary.PrintText` "Entered StartQuestTrigger!!!" true true (struct :`R` 1.0 :`B` 0.648494 :`A` 1.0) 10.0)
  (bind _asbp_player (cast `/Game/ThirdPerson/Blueprints/BP_Player` OtherActor))
  (`KismetSystemLibrary.PrintText` "CASTED TO PLAYER \n" true true (struct :`R` 0.146189 :`G` 0.213002 :`B` 1.0 :`A` 1.0) 10.0)
  (if (not (and (`self.DisableAfterStart`) (`self.WasTriggered`)))
    (`KismetSystemLibrary.PrintText` "Point is visited")
    (bind _questmanagmentsystem (`/Game/ThirdPerson/Blueprints/BP_Player.QuestManagmentSystem` _asbp_player))
    (if (`KismetSystemLibrary.IsValid` _questmanagmentsystem)
      (if (== _stepid 0)
        (bind _successed (`/Game/Source/GameInstance/BP_QuestManager.StartQuest` _questmanagmentsystem _questid))
        (if _successed
          (set `self.WasTriggered` true)
          (else
            (`KismetSystemLibrary.PrintText` "Quest not Started or aldready started" true true (struct :`R` 1.0 :`G` 0.021953 :`B` 0.020997 :`A` 1.0) 10.0)))
        (else
          (bind _succsess (`/Game/Source/GameInstance/BP_QuestManager.CompleteStep` _questmanagmentsystem _questid _stepid))
          (if _succsess
            (set `self.WasTriggered` true)
            (else
              (`KismetSystemLibrary.PrintString` "Quest Step not Completed" true true (struct :`R` 1.0 :`B` 0.025038 :`A` 1.0) 10.0))))))))

(fn `UserConstructionScript`)