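; Artifact inventory actor that holds an array of artifact instances, each with artifact data, an equipped flag and an add-to-tab flag.
; AddArtifact appends a fresh unequipped instance even for duplicates, calling the change notifier only for each existing match.
; RemoveArtifact deletes the first data match and notifies.
; ChangeArtifactForTab sets an entry's tab flag by index without notifying; all lifecycle events are empty.
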(fn `AddArtifact`
  (params (Artifact :type "/Game/Source/Inventory/S_ArtifactInstance Structure"))
  (bind (_equipped _artefactdata) (break `/Game/Source/Inventory/S_ArtifactInstance` Artifact))
  (for _array_element (`self.Artifacts`)
    (if (== (`.ArtefactData_9_41FE977F40F8361F4F28F58EC788F58E` (break `/Game/Source/Inventory/S_ArtifactInstance` _array_element)) _artefactdata)
      (`self.OnArtifactsChanged`)))
  (`KismetArrayLibrary.Array_Add` (`self.Artifacts`) (make `/Game/Source/Inventory/S_ArtifactInstance` false _artefactdata)))

(fn `ChangeArtifactForTab`
  (params (Add :type Boolean) (Index :type Integer))
  (bind _structout (setmembers `/Game/Source/Inventory/S_ArtifactInstance` :`StructRef` (`|GetArrayItem` (`self.Artifacts`) Index) :`AddToTab` Add))
  (`KismetArrayLibrary.Array_Set` (`self.Artifacts`) Index _structout))

(fn `RemoveArtifact`
  (params (Artifact :type "/Game/Source/Artifact/DA_Artifact Object Reference"))
  (for (_array_element _array_index) (`self.Artifacts`)
    (if (== Artifact (`.ArtefactData_9_41FE977F40F8361F4F28F58EC788F58E` (break `/Game/Source/Inventory/S_ArtifactInstance` _array_element)))
      (`KismetArrayLibrary.Array_Remove` (`self.Artifacts`) _array_index)
      (`self.OnArtifactsChanged`)
      (return))))

(fn `UserConstructionScript`)