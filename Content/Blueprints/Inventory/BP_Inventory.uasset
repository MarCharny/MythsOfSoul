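; BP_Inventory is an inventory Blueprint that tracks four potion counts (Damage, Health, Accuracy, Speed) and a list of artifact instances.
; Potion functions switch on type, but AddPotion leaves Speed unwired and ConsumePotion's clamped subtraction is disconnected, so it does nothing.
; AddArtifact appends unequipped, non-duplicate entries, and RemoveArtifact deletes by matching data.
; OnArtifactsChanged fires on removal or a duplicate add, but not on a new add.
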(fn `AddArtifact`
  (params (Artifact :type "/Game/Blueprints/Inventory/S_ArtifactInstance Structure"))
  (bind (_equipped _artefactdata) (break `/Game/Blueprints/Inventory/S_ArtifactInstance` Artifact))
  (for _array_element (`self.Artifacts`)
    (if (== (`.ArtefactData_9_41FE977F40F8361F4F28F58EC788F58E` (break `/Game/Blueprints/Inventory/S_ArtifactInstance` _array_element)) _artefactdata)
      (`self.OnArtifactsChanged`)
      (return)))
  (`KismetArrayLibrary.Array_Add` (`self.Artifacts`) (make `/Game/Blueprints/Inventory/S_ArtifactInstance` false _artefactdata)))

(fn `AddPotion`
  (params (Type :type "/Game/Blueprints/QuestSystem/S_PotionReward Structure"))
  (bind (_potiondata _amount) (break `/Game/Blueprints/QuestSystem/S_PotionReward` Type))
  (switch `/Game/Source/Potion/E_PotionType` (`/Game/Source/Potion/DA_Potion.PotionType` _potiondata)
    (:`NewEnumerator4`
      (setmembers `/Game/Blueprints/QuestSystem/S_PotionReward` :`StructRef` (`self.DamagePotion`) :`Amount` (+ (`.Amount_5_C8C57A634CA968D43B510F959BC6D2A8` (break `/Game/Blueprints/QuestSystem/S_PotionReward` (`self.DamagePotion`))) _amount)))
    (:`NewEnumerator1`
      (setmembers `/Game/Blueprints/QuestSystem/S_PotionReward` :`StructRef` (`self.HealthPotionCount`) :`Amount` (+ (`.Amount_5_C8C57A634CA968D43B510F959BC6D2A8` (break `/Game/Blueprints/QuestSystem/S_PotionReward` (`self.HealthPotionCount`))) _amount)))
    (:`NewEnumerator2`
      (setmembers `/Game/Blueprints/QuestSystem/S_PotionReward` :`StructRef` (`self.AccuracyPotionCount`) :`Amount` (+ (`.Amount_5_C8C57A634CA968D43B510F959BC6D2A8` (break `/Game/Blueprints/QuestSystem/S_PotionReward` (`self.AccuracyPotionCount`))) _amount)))))

(fn `ConsumePotion`
  (params (Potion :type "/Game/Blueprints/QuestSystem/S_PotionReward Structure")))

(fn `GetPotionCount`
  (params (Type :type "/Game/Source/Potion/E_PotionType Enum" :default "NewEnumerator4"))
  (returns (Count :type Integer))
  (locals (LocalCount :type Integer))
  (switch `/Game/Source/Potion/E_PotionType` Type
    (:`NewEnumerator4`
      (set `local.LocalCount` (`.Amount_5_C8C57A634CA968D43B510F959BC6D2A8` (break `/Game/Blueprints/QuestSystem/S_PotionReward` (`self.DamagePotion`)))))
    (:`NewEnumerator1`
      (set `local.LocalCount` (`.Amount_5_C8C57A634CA968D43B510F959BC6D2A8` (break `/Game/Blueprints/QuestSystem/S_PotionReward` (`self.HealthPotionCount`)))))
    (:`NewEnumerator2`
      (set `local.LocalCount` (`.Amount_5_C8C57A634CA968D43B510F959BC6D2A8` (break `/Game/Blueprints/QuestSystem/S_PotionReward` (`self.AccuracyPotionCount`)))))
    (:`NewEnumerator3`
      (set `local.LocalCount` (`.Amount_5_C8C57A634CA968D43B510F959BC6D2A8` (break `/Game/Blueprints/QuestSystem/S_PotionReward` (`self.SpeedPotionCount`))))))
  (return (`local.LocalCount`)))

(fn `RemoveArtifact`
  (params (Artifact :type "/Game/Source/Artifact/DA_Artifact Object Reference"))
  (for (_array_element _array_index) (`self.Artifacts`)
    (if (== Artifact (`.ArtefactData_9_41FE977F40F8361F4F28F58EC788F58E` (break `/Game/Blueprints/Inventory/S_ArtifactInstance` _array_element)))
      (`KismetArrayLibrary.Array_Remove` (`self.Artifacts`) _array_index)
      (`self.OnArtifactsChanged`)
      (return))))

(fn `UserConstructionScript`)