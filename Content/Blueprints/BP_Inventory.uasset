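; Inventory Blueprint that stores counts for four potion types and a duplicate-free array of artifact instances.
; AddPotion raises the change event only for Damage; ConsumePotion is empty, its clamped subtraction left unwired.
; AddArtifact appends unequipped entries but raises its change event only when the artifact already exists.
; RemoveArtifact ignores the given name, removing the first entry with ID "None" and raising the event.
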(fn `AddArtifact`
  (params (Name :type Name))
  (for _array_element (`self.Artifacts`)
    (if (== (`.ArtifactId_2_2FE371424C0715670E7F85A7924A5552` (break `/Game/Blueprints/S_ArtifactInstance` _array_element)) Name)
      (`self.OnArtifactsChanged`)
      (return)))
  (`KismetArrayLibrary.Array_Add` (`self.Artifacts`) (make `/Game/Blueprints/S_ArtifactInstance` Name)))

(fn `AddPotion`
  (params (Type :type "/Game/Source/Potion/E_PotionType Enum" :default "NewEnumerator4") (Amount :type Integer))
  (switch `/Game/Source/Potion/E_PotionType` Type
    (:`NewEnumerator4`
      (bind _output_get (set `self.DamagePotionCount` (+ (`self.DamagePotionCount`) Amount)))
      (`self.OnPotionsChanged` Type _output_get))
    (:`NewEnumerator1`
      (bind _output_get_2 (set `self.HealthPotionCount` (+ (`self.HealthPotionCount`) Amount))))
    (:`NewEnumerator2`
      (bind _output_get_3 (set `self.AccuracyPotionCount` (+ (`self.AccuracyPotionCount`) Amount))))
    (:`NewEnumerator3`
      (bind _output_get_4 (set `self.SpeedPotionCount` (+ (`self.SpeedPotionCount`) Amount))))))

(fn `ConsumePotion`
  (params (Type :type "/Game/Source/Potion/E_PotionType Enum" :default "NewEnumerator4") (Amount :type Integer)))

(fn `GetPotionCount`
  (params (Type :type "/Game/Source/Potion/E_PotionType Enum" :default "NewEnumerator4"))
  (returns (Count :type Integer))
  (locals (LocalCount :type Integer))
  (switch `/Game/Source/Potion/E_PotionType` Type
    (:`NewEnumerator4`
      (set `local.LocalCount` (`self.DamagePotionCount`)))
    (:`NewEnumerator1`
      (set `local.LocalCount` (`self.HealthPotionCount`)))
    (:`NewEnumerator2`
      (set `local.LocalCount` (`self.AccuracyPotionCount`)))
    (:`NewEnumerator3`
      (set `local.LocalCount` (`self.SpeedPotionCount`))))
  (return (`local.LocalCount`)))

(fn `RemoveArtifact`
  (params (Name :type Name))
  (for (_array_element _array_index) (`self.Artifacts`)
    (if (== (`.ArtifactId_2_2FE371424C0715670E7F85A7924A5552` (break `/Game/Blueprints/S_ArtifactInstance` _array_element)) "None")
      (`KismetArrayLibrary.Array_Remove` (`self.Artifacts`) _array_index)
      (`self.OnArtifactsChanged`)
      (return))))

(fn `UserConstructionScript`)