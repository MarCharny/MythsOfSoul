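; Game Instance quest system that tracks active and completed quests and grants their rewards.
; StartQuest checks completion and main or side prerequisites, records the quest and broadcasts OnQuestStarted, but looks up data with "None" instead of the given Id.
; CompleteQuest moves the quest to completed and adds potion and artifact rewards to the BP_Player inventory.
; GetQuestData's QuestTable row lookup is disconnected from its entry, so it never runs.
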(fn `CanStartQuest`
  (params (Id :type Name))
  (returns (CanStart :type Boolean))
  (if (`KismetArrayLibrary.Array_Contains` (`self.CompledetQuests`) Id)
    (return false)
    (else
      (bind (_found _questdata) (`self.GetQuestData` "None"))
      (if _found
        (bind (_questid _title _description _questtype _rewardsartifacts _rewardspotions _requiredmainid) (break `/Game/Blueprints/QuestSystem/S_QuestData` _questdata))
        (switch `/Game/Blueprints/QuestSystem/E_QuestType` _questtype
          (:`NewEnumerator0`
            (if (== _requiredmainid "None")
              (return true)
              (else
                (return (`KismetArrayLibrary.Array_Contains` (`self.CompledetQuests`) _requiredmainid)))))
          (:`NewEnumerator1`
            (if (== _requiredmainid "None")
              (return true)
              (else
                (return (`KismetArrayLibrary.Array_Contains` (`self.CompledetQuests`)))))))
        (else
          (return false))))))

(fn `CompleteQuest`
  (params (Id :type Name))
  (if (`KismetArrayLibrary.Array_Contains` (`self.CompledetQuests`) Id)
    (return)
    (else
      (`KismetArrayLibrary.Array_AddUnique` (`self.CompledetQuests`) Id)
      (`KismetArrayLibrary.Array_RemoveItem` (`self.ActiveQuests`) Id)
      (bind (_found _questdata) (`self.GetQuestData` Id))
      (bind _asbp_third_person_character (cast `/Game/ThirdPerson/Blueprints/BP_Player` (`GameplayStatics.GetPlayerCharacter` 0))
        (:`then`
          (bind (_questid _title _description _questtype _rewardsartifacts _rewardspotions) (break `/Game/Blueprints/QuestSystem/S_QuestData` _questdata))
          (for _array_element _rewardspotions
            (`/Game/Blueprints/Inventory/BP_Inventory.AddPotion` (`/Game/ThirdPerson/Blueprints/BP_Player.InventoryRef` _asbp_third_person_character) _array_element)
            (return))
          (bind _asbp_third_person_character_2 (cast `/Game/ThirdPerson/Blueprints/BP_Player` (`GameplayStatics.GetPlayerCharacter` 0)))
          (for _array_element_2 _rewardsartifacts
            (`/Game/Blueprints/Inventory/BP_Inventory.AddArtifact` (`/Game/ThirdPerson/Blueprints/BP_Player.InventoryRef` _asbp_third_person_character_2) _array_element_2)
            (return)))
        (:`CastFailed`
          (return))))))

(fn `GetQuestData`
  (params (Id :type Name))
  (returns (Found :type Boolean) (QuestData :type "/Game/Blueprints/QuestSystem/S_QuestData Structure")))

(fn `StartQuest`
  (params (Id :type Name))
  (bind _canstart (`self.CanStartQuest` Id))
  (if _canstart
    (if (`KismetArrayLibrary.Array_Contains` (`self.ActiveQuests`) Id)
      (return)
      (else
        (`KismetArrayLibrary.Array_AddUnique` (`self.ActiveQuests`) Id)
        (bind (_found _questdata) (`self.GetQuestData` "None"))
        (`self.OnQuestStarted` Id _questdata)))
    (else
      (return))))